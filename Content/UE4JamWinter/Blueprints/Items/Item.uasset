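; Purchasable item actor that offers one of three boosts (max health, heal or attack) for a coin price.
; On BeginPlay it builds the boost text, shows the price and picks a Paper2D flipbook matching the boost type.
; Bought and CannotAfford events only handle feedback: a purchase shows the boost, marks the item used, blanks the sprite and destroys it after a delay.
; A failed purchase briefly shows a warning before restoring the price.
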(event Custom|Bought
  ;[0.01124 0.6667 0] Bought
  (Rendering|Components|TextRender|SetText (Variables|Default|GetDescriptionDisplayed) (Variables|Text|GetBoostDescription))
  (Variables|Default|SetUsed true)
  (Sprite|SetFlipbook (Variables|Default|GetImage) "/Game/UE4JamWinter/Blueprints/Items/blank_Flipbook.blank_Flipbook")
  (Utilities|FlowControl|Delay 2.0)
  (Actor|DestroyActor))

(event Custom|Cannot%20Afford
  ;[0.6649 0 0.01614] Cannot Afford
  (Rendering|Components|TextRender|SetText (Variables|Default|GetDescriptionDisplayed) (Variables|Text|GetCannotAffordDescription))
  (Utilities|FlowControl|Delay 2.0)
  (Rendering|Components|TextRender|SetText (Variables|Default|GetDescriptionDisplayed) (Utilities|Text|ToText(String) (Utilities|String|Append (Utilities|String|ToString(Integer) (Variables|Default|GetPrice)) " Coins"))))

(event EventBeginPlay
  ;[0.1836 0 0.6453] Begin Play
  (Variables|Text|SetBoostDescription (Utilities|Text|ToText(String) (Utilities|String|Append "+" (Utilities|String|ToString(Float) (Variables|Default|GetBoostQuantity)) " " (Utilities|Select :Index (Variables|Default|GetBoostType) :NewEnumerator0 "Max Health" :NewEnumerator1 "HP" :NewEnumerator2 "Attack") " !")))
  (Rendering|Components|TextRender|SetText (Variables|Default|GetDescriptionDisplayed) (Utilities|Text|ToText(String) (Utilities|String|Append (Utilities|String|ToString(Integer) (Variables|Default|GetPrice)) " Coins")))
  (switch Utilities|FlowControl|Switch|SwitchonItemType (Variables|Default|GetBoostType)
    (:NewEnumerator0
      (Sprite|SetFlipbook (Variables|Default|GetImage) "/Game/UE4JamWinter/Sprites/Items/MaxHealthPotion.MaxHealthPotion"))
    (:NewEnumerator1
      (Sprite|SetFlipbook (Variables|Default|GetImage) "/Game/UE4JamWinter/Sprites/Items/Heal.Heal"))
    (:NewEnumerator2
      (Sprite|SetFlipbook (Variables|Default|GetImage) "/Game/UE4JamWinter/Sprites/Items/StrengthPotion.StrengthPotion"))))

(fn ConstructionScript)