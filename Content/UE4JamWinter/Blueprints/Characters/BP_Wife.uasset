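; BP_Wife is a 2D flipbook companion character that follows the player along the X axis.
; Overlap with the LimitFollow component stops following when the player enters and resumes it when they leave.
; While following, Tick feeds the X offset to the player into movement input and plays the walk flipbook, otherwise idle.
; Yaw flips with X velocity, falling back to the player's side when velocity is zero.
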(event OnComponentBeginOverlap(LimitFollow)
  (params (OverlappedComponent :type Primitive%20Component%20Object%20Reference) (OtherActor :type Actor%20Object%20Reference) (OtherComp :type Primitive%20Component%20Object%20Reference) (OtherBodyIndex :type Integer) (bFromSweep :type Boolean) (SweepResult :type Hit%20Result%20Structure%20%28by%20ref%29))
  (Utilities|Casting|CastToBP_MainCharacter OtherActor)
  (Variables|Default|SetFollow false))

(event OnComponentEndOverlap(LimitFollow)
  (params (OverlappedComponent :type Primitive%20Component%20Object%20Reference) (OtherActor :type Actor%20Object%20Reference) (OtherComp :type Primitive%20Component%20Object%20Reference) (OtherBodyIndex :type Integer))
  (Utilities|Casting|CastToBP_MainCharacter OtherActor)
  (Variables|Default|SetFollow true))

(event EventTick
  (params (DeltaSeconds :type Float%20%28single-precision%29))
  (bind _capsulecomponent (Variables|Collision|GetCapsuleComponent))
  (bind _returnvalue (Transformation|GetWorldLocation _capsulecomponent))
  (if (Variables|Default|GetFollow)
    (bind _asbp_main_character (Utilities|Casting|CastToBP_MainCharacter (Game|GetPlayerCharacter 0)))
    (Variables|Default|SetbisMovingRight (> (.x (Transformation|GetWorldLocation (Variables|/Script/Engine.Character|GetCapsuleComponent _asbp_main_character))) (.x _returnvalue)))
    (Pawn|Input|AddMovementInput "1.000000, 0, 0" (- (.x (Transformation|GetWorldLocation (Variables|/Script/Engine.Character|GetCapsuleComponent _asbp_main_character))) (.x _returnvalue)) false)
    (Sprite|SetFlipbook (Variables|Default|GetSprite) (Variables|Default|GetFB%20Walk))
    (Math|Float|CompareFloat (.X (Math|Vector|BreakVector (Variables|/Script/Engine.MovementComponent|GetVelocity (Pawn|GetMovementComponent)))) 0.0
      (:>
        (Transformation|SetActorRotation (Math|Rotator|MakeRotator 0.0 0.0 0.0) :!label _label))
      (:==
        (if (Variables|Default|GetbisMovingRight)
          (goto _label)
          (else
            (Transformation|SetActorRotation (Math|Rotator|MakeRotator 0.0 0.0 1.8e+02) :!label _label_2))))
      (:<
        (goto _label_2)))
    (else
      (Sprite|SetFlipbook (Variables|Default|GetSprite) "/Game/UE4JamWinter/Sprites/Characters/Wife/Wife_Idle.Wife_Idle"))))

(fn ConstructionScript)