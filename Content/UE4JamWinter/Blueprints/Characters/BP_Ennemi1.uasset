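; BP_Ennemi1 is a 2D flipbook character using Light Bandit animations, driven by player movement, jump and touch input despite its enemy name.
; On BeginPlay it sets the sprite component to replicate.
; Each Tick switches between run and idle flipbooks by speed and flips control yaw by horizontal velocity.
; When horizontal velocity is zero, the last MoveRight input direction, stored in BisMovingRight, keeps the facing.
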(event Custom|UpdateAnimation
  ;[0.1643 0.657 0] Handle Animation
  (Sprite|SetFlipbook (Variables|Default|GetSprite) (select (> (Math|Vector|VectorLength (Transformation|GetVelocity)) 0.0) "/Game/UE4JamWinter/Animations/T_LightBandit_RUN.T_LightBandit_RUN" "/Game/UE4JamWinter/Animations/T_LightBandit_IDLE.T_LightBandit_IDLE")))

(event EventTick
  (params (DeltaSeconds :type Float%20%28single-precision%29))
  ;[0 0.5991 0.2222] Tick - Updates animation
  (CallFunction|UpdateAnimation)
  (Math|Float|CompareFloat (.X (Math|Vector|BreakVector (Variables|/Script/Engine.MovementComponent|GetVelocity (Pawn|GetMovementComponent)))) 0.0
    (:>
      (Pawn|SetControlRotation (Pawn|GetController) (Math|Rotator|MakeRotator 0.0 0.0 1.8e+02) :!label _label))
    (:==
      (if (Variables|Default|GetbisMovingRight)
        (goto _label)
        (else
          (Pawn|SetControlRotation (Pawn|GetController) (Math|Rotator|MakeRotator 0.0 0.0 0.0) :!label _label_2))))
    (:<
      (goto _label_2))))

(event EventBeginPlay
  (Class|ActorComponent|SetIsReplicated (Variables|Default|GetSprite) true))

(event Input|ActionEvents|InputActionJump
  (params (Key :type Key%20Structure))
  ;[0 0.657 0.1643] Handle Jump
  (:Pressed
    (Character|Jump))
  (:Released
    (Character|StopJumping)))

(event Input|AxisEvents|InputAxisMoveRight
  (params (AxisValue :type Float%20%28single-precision%29))
  ;[0.773 0 0.04889] Handle movement
  (if (> AxisValue 0.0)
    (Variables|Default|SetbisMovingRight true)
    (elif (< AxisValue 0.0)
      (Variables|Default|SetbisMovingRight false)))
  (Pawn|Input|AddMovementInput "1.000000, 0, 0" AxisValue false))

(event Input|TouchEvents|InputTouch
  (params (Location :type Vector) (FingerIndex :type ETouchIndex%20Enum))
  ;[0 0.657 0.1643] Handle Jump
  (:Pressed
    (Character|Jump))
  (:Released
    (Character|StopJumping)))

(fn ConstructionScript)