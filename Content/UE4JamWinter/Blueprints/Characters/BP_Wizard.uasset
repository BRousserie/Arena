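; BP_Wizard is a Paper2D flipbook character that reacts when the main character comes near.
; Capsule overlap with BP_MainCharacter plays a take-fire animation, then switches to a looping idle.
; When that overlap ends, it plays a take-off-fire animation, then returns to the default idle.
; Each transition is timed by a Delay equal to the flipbook's length.
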(event OnComponentBeginOverlap(CapsuleComponent)
  (params (OverlappedComponent :type Primitive%20Component%20Object%20Reference) (OtherActor :type Actor%20Object%20Reference) (OtherComp :type Primitive%20Component%20Object%20Reference) (OtherBodyIndex :type Integer) (bFromSweep :type Boolean) (SweepResult :type Hit%20Result%20Structure%20%28by%20ref%29))
  (Utilities|Casting|CastToBP_MainCharacter OtherActor)
  (Sprite|SetFlipbook (Variables|Default|GetSprite) "/Game/UE4JamWinter/Sprites/Characters/Seller/wizard_idle_Sprite_WizardTakeFire.wizard_idle_Sprite_WizardTakeFire")
  (Utilities|FlowControl|Delay (Class|PaperFlipbookComponent|GetFlipbookLength (Variables|Default|GetSprite)))
  (Sprite|SetFlipbook (Variables|Default|GetSprite) "/Game/UE4JamWinter/Sprites/Characters/Seller/wizard_idle_Sprite_WizarIdIeLoop.wizard_idle_Sprite_WizarIdIeLoop"))

(event OnComponentEndOverlap(CapsuleComponent)
  (params (OverlappedComponent :type Primitive%20Component%20Object%20Reference) (OtherActor :type Actor%20Object%20Reference) (OtherComp :type Primitive%20Component%20Object%20Reference) (OtherBodyIndex :type Integer))
  (Utilities|Casting|CastToBP_MainCharacter OtherActor)
  (Sprite|SetFlipbook (Variables|Default|GetSprite) "/Game/UE4JamWinter/Sprites/Characters/Seller/wizard_idle_Sprite_WizardTakeOffFire.wizard_idle_Sprite_WizardTakeOffFire")
  (Utilities|FlowControl|Delay (Class|PaperFlipbookComponent|GetFlipbookLength (Variables|Default|GetSprite)))
  (Sprite|SetFlipbook (Variables|Default|GetSprite) "/Game/UE4JamWinter/Sprites/Characters/Seller/wizard_idle_Sprite_WizardIdle.wizard_idle_Sprite_WizardIdle"))

(event Collision|EventActorBeginOverlap
  (params (OtherActor :type Actor%20Object%20Reference)))

(event EventTick
  (params (DeltaSeconds :type Float%20%28single-precision%29)))

(fn ConstructionScript)