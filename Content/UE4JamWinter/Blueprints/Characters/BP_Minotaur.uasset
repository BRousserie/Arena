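; BP_Minotaur is a 2D sprite fighter character whose attack and idle animation change at half health.
; AtkSword runs a circle attack through FighterComp at half health or above, and a sword attack below it, each with its own collision shape.
; GetIdle swaps idle animations around that threshold.
; RotateSprite flips actor yaw for negative or zero X velocity, consulting IsMovingRight_2 when stationary; positive velocity is unhandled.
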(event EventAtkSword
  (bind _fightercomp (Variables|Default|GetFighterComp))
  (if (>= (Variables|/Game/UE4JamWinter/Blueprints/Characters/FighterComp.FighterComp_C|GetHealth _fightercomp) (/ (Variables|/Game/UE4JamWinter/Blueprints/Characters/FighterComp.FighterComp_C|GetMaxHealth _fightercomp) 2.0))
    (Default|Attack (Variables|Default|GetFighterComp) (Variables|Default|GetCircleAttack) (Variables|Default|GetCircleRange) self)
    (else
      (Default|Attack (Variables|Default|GetFighterComp) (Variables|Default|GetSwordAttack) (Variables|Default|GetSwordRange) self))))

(event EventRotateSprite
  (Math|Float|CompareFloat (.X (Math|Vector|BreakVector (Variables|/Script/Engine.MovementComponent|GetVelocity (Pawn|GetMovementComponent)))) 0.0
    (:==
      (if (|isMovingRight_2)
        (Transformation|SetActorRotation (Math|Rotator|MakeRotator 0.0 0.0 0.0))
        (else
          (Transformation|SetActorRotation (Math|Rotator|MakeRotator 0.0 0.0 1.8e+02) :!label _label))))
    (:<
      (goto _label))))

(fn ConstructionScript
  (|CallParentFunction))

(fn GetIdle
  (bind _fightercomp (Variables|Default|GetFighterComp))
  (if (> (Variables|/Game/UE4JamWinter/Blueprints/Characters/FighterComp.FighterComp_C|GetHealth _fightercomp) (/ (Variables|/Game/UE4JamWinter/Blueprints/Characters/FighterComp.FighterComp_C|GetMaxHealth _fightercomp) 2.0))
    (return "/Game/UE4JamWinter/Animations/Minotaur_IDLE.Minotaur_IDLE")
    (else
      (return "/Game/UE4JamWinter/Animations/Minotaur_IDLE2.Minotaur_IDLE2"))))