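; Generic 2D side-scroller enemy AI that chases, attacks and guards against the player using flipbook animations.
; Tick picks death, falling, attack, guard, chase or idle in priority order, using sight and sword-range overlap flags, and sets facing.
; A recursive random timer toggles guarding, with longer possible gaps when the player is farther away.
; FighterComp handles attacks, while death plays once, notifies the game mode and destroys the actor.
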(event Custom|atkSword
  ;[0 0.3575 0.4638] Actions
  (Default|Attack (Variables|Default|GetFighterComp) (Variables|Default|GetSwordAttack) (Variables|Default|GetSwordRange) self))

(event Custom|guard
  ;[0 0.3575 0.4638] Actions
  (Sprite|SetFlipbook (Variables|Default|GetSprite) (Variables|FlipBooks|GetFB_GUARD))
  (Components|Movement|StopMovementImmediately (Variables|Character|GetCharacterMovement)))

(event Custom|RandomlyGuard
  ;[0.3285 0 0.4987] Make AI Guard randomly
  (Utilities|FlowControl|Delay (Math|Random|RandomFloatinRange 0.2 (/ (Transformation|GetDistanceTo (Game|GetPlayerCharacter 0)) 3e+02)))
  (Variables|BehaviourInfos|SetshouldGuard true)
  (Utilities|FlowControl|Delay (Math|Random|RandomFloatinRange 0.2 1.5))
  (Variables|BehaviourInfos|SetshouldGuard false)
  (CallFunction|RandomlyGuard))

(event Custom|moveToPlayer
  (bind _capsulecomponent (Variables|Collision|GetCapsuleComponent))
  (bind _returnvalue (Transformation|GetWorldLocation _capsulecomponent))
  ;[0 0.3575 0.4638] Actions
  (bind _asbp_main_character (Utilities|Casting|CastToBP_MainCharacter (Game|GetPlayerCharacter 0)))
  (Variables|/Game/UE4JamWinter/Blueprints/Characters/FighterComp.FighterComp_C|SetisMovingRight (Variables|Default|GetFighterComp self) (> (.x (Transformation|GetWorldLocation (Variables|/Script/Engine.Character|GetCapsuleComponent _asbp_main_character))) (.x _returnvalue)))
  (Pawn|Input|AddMovementInput "1.000000, 0, 0" (- (.x (Transformation|GetWorldLocation (Variables|/Script/Engine.Character|GetCapsuleComponent _asbp_main_character))) (.x _returnvalue)) false)
  (Sprite|SetFlipbook (Variables|Default|GetSprite) (Variables|FlipBooks|GetFB_RUN)))

(event Custom|falling
  ;[0 0.3575 0.4638] Actions
  (Sprite|SetFlipbook (Variables|Default|GetSprite) (Variables|FlipBooks|GetFB_JUMP)))

(event Custom|die
  (bind _fb_dying (Variables|FlipBooks|GetFB_DYING))
  ;[0 0.3575 0.4638] Actions
  (Utilities|FlowControl|DoOnce false
    (:Completed
      (Sprite|SetFlipbook (Variables|Default|GetSprite) _fb_dying)
      (Utilities|FlowControl|Delay (Class|PaperFlipbook|GetTotalDuration _fb_dying))
      (Sprite|SetFlipbook (Variables|Default|GetSprite) (Variables|FlipBooks|GetFB_DEAD))
      (Collision|SetCollisionEnabled (Variables|Collision|GetCapsuleComponent) "NoCollision")
      (Utilities|FlowControl|Delay 1.0)
      (Default|AIDeath (.AsBP%202DSide%20Scroller%20Game%20Mode (Utilities|Casting|CastToBP_2DSideScrollerGameMode (Game|GetGameMode))))
      (Actor|DestroyActor))))

(event EventBeginPlay
  ;[0.3285 0 0.4987] Make AI Guard randomly
  (CallFunction|RandomlyGuard)
  (Variables|BehaviourInfos|SetisOverlapping true))

(event EventTick
  (params (DeltaSeconds :type Float%20%28single-precision%29))
  ;[0 0.5991 0.2222] Tick - Decision center
  (if (not (Variables|/Game/UE4JamWinter/Blueprints/Characters/FighterComp.FighterComp_C|GetisAttacking (Variables|Default|GetFighterComp self)))
    (if (|isDead)
      (CallFunction|Die)
      (else
        (if (AI|Components|NavMovement|IsFalling (Variables|Character|GetCharacterMovement))
          (CallFunction|Falling)
          (elif (Variables|BehaviourInfos|GetisOverlappingSword)
            (CallFunction|AtkSword)
            (elif (Variables|BehaviourInfos|GetshouldGuard)
              (CallFunction|Guard)
              (elif (Variables|BehaviourInfos|GetisOverlapping)
                (CallFunction|MovetoPlayer)
                (else
                  (Sprite|SetFlipbook (Variables|Default|GetSprite) (Variables|FlipBooks|GetFB_IDLE)))))))
        (Math|Float|CompareFloat (.X (Math|Vector|BreakVector (Variables|/Script/Engine.MovementComponent|GetVelocity (Pawn|GetMovementComponent)))) 0.0
          (:>
            (Transformation|SetActorRotation (Math|Rotator|MakeRotator 0.0 0.0 1.8e+02) :!label _label))
          (:==
            (if (|isMovingRight)
              (goto _label)
              (else
                (Transformation|SetActorRotation (Math|Rotator|MakeRotator 0.0 0.0 0.0) :!label _label_2))))
          (:<
            (goto _label_2)))))))

(event OnComponentBeginOverlap(Sight)
  (params (OverlappedComponent :type Primitive%20Component%20Object%20Reference) (OtherActor :type Actor%20Object%20Reference) (OtherComp :type Primitive%20Component%20Object%20Reference) (OtherBodyIndex :type Integer) (bFromSweep :type Boolean) (SweepResult :type Hit%20Result%20Structure%20%28by%20ref%29))
  ;[0.02899 0 0.8018] Sight Overlap Events
  (if (Components|ComponentHasTag OtherComp "Player")
    (Variables|BehaviourInfos|SetisOverlapping true)))

(event OnComponentEndOverlap(Sight)
  (params (OverlappedComponent :type Primitive%20Component%20Object%20Reference) (OtherActor :type Actor%20Object%20Reference) (OtherComp :type Primitive%20Component%20Object%20Reference) (OtherBodyIndex :type Integer))
  ;[0.02899 0 0.8018] Sight Overlap Events
  (if (Components|ComponentHasTag OtherComp "Player")
    (Variables|BehaviourInfos|SetisOverlapping false)))

(event OnComponentBeginOverlap(SwordRange)
  (params (OverlappedComponent :type Primitive%20Component%20Object%20Reference) (OtherActor :type Actor%20Object%20Reference) (OtherComp :type Primitive%20Component%20Object%20Reference) (OtherBodyIndex :type Integer) (bFromSweep :type Boolean) (SweepResult :type Hit%20Result%20Structure%20%28by%20ref%29))
  ;[0.7537 0.06764 0] Sword Overlap Events
  (if (Components|ComponentHasTag OtherComp "Player")
    (Variables|BehaviourInfos|SetisOverlappingSword true)))

(event OnComponentEndOverlap(SwordRange)
  (params (OverlappedComponent :type Primitive%20Component%20Object%20Reference) (OtherActor :type Actor%20Object%20Reference) (OtherComp :type Primitive%20Component%20Object%20Reference) (OtherBodyIndex :type Integer))
  ;[0.7537 0.06764 0] Sword Overlap Events
  (if (Components|ComponentHasTag OtherComp "Player")
    (Variables|BehaviourInfos|SetisOverlappingSword false)))

(fn ConstructionScript)