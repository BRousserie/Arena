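; BP_GameArena is an unfinished arena round manager for bandit and minotaur waves.
; CalculateEnnemiesAtRound derives per-type enemy counts from rounds won, and PickRandomAIClass uses them for a weighted random class choice.
; AIDeath is meant to spawn replacements at two locations or open the intermission level when no enemies remain, but that logic is disconnected.
; CountDeaths and the event graph are empty.
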(event EventBeginPlay)

(event EventTick
  (params (DeltaSeconds :type Float%20%28single-precision%29)))

(fn ConstructionScript)

(fn AIDeath
  (params (SlayedEntityClass :type String)))

(fn CalculateEnnemiesatRound
  (Variables|UE4JAM|SetLightBanditsToSpawn_ROUND (* 2 (Variables|Default|GetRoundsWon)))
  (Variables|UE4JAM|SetHeavyBanditsToSpawn_ROUND (Variables|Default|GetRoundsWon))
  (Variables|UE4JAM|SetMinotaursToSpawn_ROUND (/ 3 (Variables|Default|GetRoundsWon))))

(fn PickRandomAIClass
  (bind _lightbanditstospawn_round (Variables|UE4JAM|GetLightBanditsToSpawn_ROUND))
  (bind _ennemiestodefeat_round (Variables|UE4JAM|GetEnnemiesToDefeat_ROUND))
  (bind _returnvalue (Math|Random|RandomInteger _ennemiestodefeat_round))
  (if (< _returnvalue _lightbanditstospawn_round)
    (bind _class_ (Class|LowEntryExtendedStandardLibrary|GetClasswithName (Variables|Default|GetLightBanditClassName)))
    (bind _aspawn (Utilities|Casting|CastToPawnClass _class_))
    (return _aspawn)
    (elif (< _returnvalue (+ _lightbanditstospawn_round (Variables|UE4JAM|GetHeavyBanditsToSpawn_ROUND)))
      (bind _class__2 (Class|LowEntryExtendedStandardLibrary|GetClasswithName (Variables|Default|GetHeavyBanditClassName)))
      (bind _aspawn_2 (Utilities|Casting|CastToPawnClass _class__2))
      (return _aspawn_2)
      (else
        (bind _class__3 (Class|LowEntryExtendedStandardLibrary|GetClasswithName (Variables|Default|GetMinotaurClassName)))
        (bind _aspawn_3 (Utilities|Casting|CastToPawnClass _class__3))
        (return _aspawn_3)))))

(fn CountDeaths)