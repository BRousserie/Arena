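; Fighter component that handles melee attacks, health and death for the main character and generic enemies in a Paper2D game.
; Attack plays the attack's flipbook, waits for its hit time, then gathers player and enemy pawns overlapping the attack shape, excluding the attacker.
; Each target's own FighterComp takes damage and signals pawn death, and the target is launched by a direction-aware knockback.
; Done clears IsAttacking after the remaining animation time.
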(event Custom|done
  (bind _attackaction (Variables|Default|GetAttackAction))
  ;[0 0.2512 0.5701] Finish Attack
  (Utilities|FlowControl|Delay (- (Class|PaperFlipbook|GetTotalDuration (Variables|/Game/UE4JamWinter/Blueprints/AttackComp.AttackComp_C|GetAnimation _attackaction)) (Variables|/Game/UE4JamWinter/Blueprints/AttackComp.AttackComp_C|GetHitTime _attackaction)))
  (Variables|BehaviourInfos|SetisAttacking false))

(event Custom|Attack
  (params (Attack :type Attack%20Comp%20Object%20Reference) (AttackCollisionShape :type Shape%20Component%20Object%20Reference) (Attacker :type Paper%20Character%20Object%20Reference))
  ;[0.7923 0 0.02933] Start Attack
  (bind _output_get (Variables|Default|SetAttackAction Attack))
  (Sprite|SetFlipbook (Variables|/Script/Paper2D.PaperCharacter|GetSprite Attacker) (Variables|/Game/UE4JamWinter/Blueprints/AttackComp.AttackComp_C|GetAnimation _output_get))
  (Variables|BehaviourInfos|SetisAttacking true)
  (Utilities|FlowControl|Delay (Variables|/Game/UE4JamWinter/Blueprints/AttackComp.AttackComp_C|GetHitTime (Variables|Default|GetAttackAction)))
  ;[0.03865 0 0.792] Loop over Overlapped Actors
  (bind _targets (CallFunction|GetOverlappedActors AttackCollisionShape Attacker))
  (for _array_element _targets
    (bind _asbp_generic_ennemy (Utilities|Casting|CastToBP_Generic_Ennemy _array_element)
      (:then
        _)
      (:CastFailed
        (bind _asbp_main_character (Utilities|Casting|CastToBP_MainCharacter _array_element))))
    (bind _valid (CallFunction|GetValidTarget _asbp_generic_ennemy _asbp_main_character))
    (Utilities|IsValid _valid
      (:Is%20Valid
        ;[0.2995 0.5218 0] Apply Attack Effects
        (CallFunction|DealDamages _valid (Variables|/Game/UE4JamWinter/Blueprints/AttackComp.AttackComp_C|GetStrength (Variables|Default|GetAttackAction)))
        (bind _aspaper_character (Utilities|Casting|CastToPaperCharacter _array_element))
        (CallFunction|KnockBack _aspaper_character (Variables|/Game/UE4JamWinter/Blueprints/AttackComp.AttackComp_C|GetKnockBackVector (Variables|Default|GetAttackAction)) (Variables|BehaviourInfos|GetisMovingRight))
        (CallFunction|Done))))
  (CallFunction|Done))

(fn DealDamages
  (params (Strength :type Float%20%28single-precision%29))
  (bind _output_get (Variables|Stats|SetHealth (- (Variables|Stats|GetHealth) Strength)))
  (Variables|BehaviourInfos|SetisDead (< _output_get 0.0))
  (Default|CallPawnDies))

(fn GetOverlappedActors
  (params (ShapeCollision :type Shape%20Component%20Object%20Reference) (NewParam :type Actor%20Object%20Reference))
  (bind _array (Utilities|Array|MakeArray NewParam))
  (Utilities|IsValid ShapeCollision
    (:Is%20Valid
      (bind _outactors (Collision|ComponentOverlapActors ShapeCollision (Transformation|GetWorldTransform ShapeCollision) (Utilities|Array|MakeArray "ObjectTypeQuery3") "/Game/UE4JamWinter/Blueprints/Characters/MainCharacter/BP_MainCharacter.BP_MainCharacter_C" _array))
      (bind _outactors_2 (Collision|ComponentOverlapActors ShapeCollision (Transformation|GetWorldTransform ShapeCollision) (Utilities|Array|MakeArray "ObjectTypeQuery3") "/Game/UE4JamWinter/Blueprints/Characters/BP_Generic_Ennemy.BP_Generic_Ennemy_C" _array))
      (Utilities|Array|AppendArray _outactors _outactors_2)
      (return _outactors))
    (:Is%20Not%20Valid
      (return 0))))

(fn GetValidTarget
  (params (Target1 :type BP%20Generic%20Ennemy%20Object%20Reference) (Target2 :type BP%20Main%20Character%20Object%20Reference))
  (Utilities|IsValid Target1
    (:Is%20Valid
      (return (Variables|/Game/UE4JamWinter/Blueprints/Characters/BP_Generic_Ennemy.BP_Generic_Ennemy_C|GetFighterComp Target1)))
    (:Is%20Not%20Valid
      (Utilities|IsValid Target2
        (:Is%20Valid
          (return (Variables|/Game/UE4JamWinter/Blueprints/Characters/MainCharacter/BP_MainCharacter.BP_MainCharacter_C|GetFighterComp Target2)))
        (:Is%20Not%20Valid
          (return 0))))))

(fn KnockBack
  (params (Target :type Paper%20Character%20Object%20Reference) (Ratio :type Vector) (Right :type Boolean))
  (Character|LaunchCharacter Target (* Ratio (Math|Vector|MakeVector (select Right 1.0 -1.0) 0.0 1.0)) false false))