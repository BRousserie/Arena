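; SpawnVolumeSurvie is a box volume that spawns enemy AI for the Survival game mode.
; On BeginPlay it has BP_Survival calculate the round's enemy count, registers itself there, then triggers SpawnAIs after a short delay.
; SpawnAI spawns the given class at a random point along the box's world X extent, centered on the actor, adjusting for collisions but always spawning.
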(event EventBeginPlay
  (bind _returnvalue (Game|GetGameMode))
  (bind _asbp_survival (Utilities|Casting|CastToBP_Survival _returnvalue))
  (Default|CalculateEnnemiesatRound _asbp_survival)
  (Default|InitSpawnVolume _asbp_survival self)
  (Utilities|FlowControl|Delay 0.2)
  (Default|SpawnAIs _asbp_survival))

(fn ConstructionScript)

(fn SpawnAI
  (params (EnnemyClass :type Pawn%20Class%20Reference))
  (bind _spawnarea (Variables|Default|GetSpawnArea))
  (bind _returnvalue (Components|Box|GetScaledBoxExtent _spawnarea))
  (Game|SpawnActorfromClass EnnemyClass (Math|Transform|MakeTransform (+ (Math|Vector|MakeVector (Math|Random|RandomFloatinRange (* (.x _returnvalue) -1.0) (.x _returnvalue)) 0.0 0.0) (Transformation|GetActorLocation))) "AdjustIfPossibleButAlwaysSpawn" 0 0))