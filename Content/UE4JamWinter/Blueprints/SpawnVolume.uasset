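; SpawnVolume is a placed actor that spawns enemy AI in the 2D side-scroller.
; On BeginPlay it has BP_2DSideScrollerGameMode calculate the round's enemy count, registers itself with it and triggers SpawnAIs.
; SpawnAI spawns a given enemy class at a random X offset within the SpawnArea box, keeping the volume's Y and Z and adjusting for collisions but always spawning.
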(event EventBeginPlay
  (bind _returnvalue (Game|GetGameMode))
  (bind _asbp_2dside_scroller_game_mode (Utilities|Casting|CastToBP_2DSideScrollerGameMode _returnvalue))
  (Default|CalculateEnnemiesatRound _asbp_2dside_scroller_game_mode)
  (Default|InitSpawnVolume _asbp_2dside_scroller_game_mode self)
  (Default|SpawnAIs _asbp_2dside_scroller_game_mode))

(fn ConstructionScript)

(fn SpawnAI
  (params (EnnemyClass :type Pawn%20Class%20Reference))
  (bind _spawnarea (Variables|Default|GetSpawnArea))
  (bind _returnvalue (Components|Box|GetScaledBoxExtent _spawnarea))
  (Game|SpawnActorfromClass EnnemyClass (Math|Transform|MakeTransform (+ (Math|Vector|MakeVector (Math|Random|RandomFloatinRange (* (.x _returnvalue) -1.0) (.x _returnvalue)) 0.0 0.0) (Transformation|GetActorLocation))) "AdjustIfPossibleButAlwaysSpawn" 0 0))