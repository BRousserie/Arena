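; Survival-mode manager that spawns bandit and minotaur enemies and tracks kills and score.
; Tick uses a Delay that shortens with kills to spawn a weighted-random enemy class in one of two spawn areas.
; Round number sets the enemy mix and stage cap, though the loop filling to that cap is unconnected.
; AIDeath updates counters and adds combo-multiplied score to the game instance.
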(event EventTick
  (params (DeltaSeconds :type Float%20%28single-precision%29))
  (Utilities|FlowControl|Delay (+ (/ 5.0 (+ (Math|Conversions|ToFloat(Integer) (Variables|UE4JAM|GetEnnemiesDefeated)) 1.0)) 5.0))
  (bind _aiclass (CallFunction|PickRandomAIClass))
  (if (== (Math|Random|RandomInteger 2) 1)
    (Default|SpawnAI (Variables|Default|GetSpawnArea) _aiclass)
    (else
      (Default|SpawnAI (Variables|Default|GetSpawnArea2) _aiclass))))

(fn ConstructionScript)

(fn AIDeath
  (params (Ennemi :type BP%20Generic%20Ennemy%20Object%20Reference))
  (CallFunction|CalculateScore (Variables|/Game/UE4JamWinter/Blueprints/Characters/BP_Generic_Ennemy.BP_Generic_Ennemy_C|GetValue Ennemi))
  (CallFunction|CountDeaths))

(fn CalculateEnnemiesatRound
  (bind _roundnumber (Utilities|GameRoundNumber))
  (bind _roundnumber_2 (Utilities|GameRoundNumber))
  (bind _output_get (Variables|UE4JAM|SetLightBanditsToSpawn (* 3 _roundnumber_2)))
  (bind _output_get_2 (Variables|UE4JAM|SetHeavyBanditsToSpawn (* _roundnumber_2 2)))
  (bind _output_get_3 (Variables|UE4JAM|SetMinotaursToSpawn _roundnumber_2))
  (Variables|UE4JAM|SetEnnemiesToDefeat (+ _output_get_2 _output_get _output_get_3))
  (Variables|UE4JAM|SetMaxEnnemiesOnStage (+ (Math|Float|Truncate (+ (/ (Math|Conversions|ToFloat(Integer) _roundnumber) 2.0) (Math|Float|Sqrt (Math|Conversions|ToFloat(Integer) _roundnumber)))) (+ _roundnumber 1))))

(fn PickRandomAIClass
  (bind _lightbanditstospawn (Variables|UE4JAM|GetLightBanditsToSpawn))
  (bind _ennemiestodefeat (Variables|UE4JAM|GetEnnemiesToDefeat))
  (bind _returnvalue (Math|Random|RandomInteger _ennemiestodefeat))
  (if (< _returnvalue _lightbanditstospawn)
    (return "/Game/UE4JamWinter/Blueprints/Characters/BP_LightBandit.BP_LightBandit_C")
    (elif (< _returnvalue (+ _lightbanditstospawn (Variables|UE4JAM|GetHeavyBanditsToSpawn)))
      (return "/Game/UE4JamWinter/Blueprints/Characters/BP_HeavyBandit.BP_HeavyBandit_C")
      (else
        (return "/Game/UE4JamWinter/Blueprints/Characters/BP_Minotaur.BP_Minotaur_C")))))

(fn CountDeaths
  (Math|Integer|IncrementInt (Variables|UE4JAM|GetEnnemiesDefeated)
    (:%20%20
      (Math|Integer|IncrementInt (Variables|/Game/UE4JamWinter/Blueprints/UE4JamGameInstance.UE4JamGameInstance_C|GetennemiesDefeated (.AsUE4Jam%20Game%20Instance (Utilities|Casting|CastToUE4JamGameInstance (Game|GetGameInstance))))
        (:%20%20
          (Math|Integer|DecrementInt (Variables|UE4JAM|GetEnnemiesOnStage)
            (:%20%20
              (Math|Integer|DecrementInt (Variables|UE4JAM|GetEnnemiesToDefeat)))))))))

(fn InitSpawnVolume
  (params (SpawnArea :type Spawn%20Volume%20Survie%20Object%20Reference))
  (if (Utilities|IsValid (Variables|Default|GetSpawnArea))
    (Variables|Default|SetSpawnArea2 SpawnArea)
    (else
      (Variables|Default|SetSpawnArea SpawnArea))))

(fn SpawnAIs
  (if (and (Utilities|IsValid (Variables|Default|GetSpawnArea)) (Utilities|IsValid (Variables|Default|GetSpawnArea2)))
    (bind _aiclass (CallFunction|PickRandomAIClass))
    (if (== (Math|Random|RandomInteger 2) 1)
      (Default|SpawnAI (Variables|Default|GetSpawnArea2) _aiclass)
      (else
        (Default|SpawnAI (Variables|Default|GetSpawnArea) _aiclass)))
    (Math|Integer|IncrementInt (Variables|UE4JAM|GetEnnemiesOnStage))))

(fn CalculateScore
  (params (Value :type Float%20%28single-precision%29))
  (bind _returnvalue (Game|GetGameInstance))
  (bind _asue4jam_game_instance (Utilities|Casting|CastToUE4JamGameInstance _returnvalue))
  (Variables|/Game/UE4JamWinter/Blueprints/UE4JamGameInstance.UE4JamGameInstance_C|Setscore _asue4jam_game_instance (+ (* Value (Variables|UE4JAM|GetComboMultiplicator)) (Variables|/Game/UE4JamWinter/Blueprints/UE4JamGameInstance.UE4JamGameInstance_C|Getscore _asue4jam_game_instance))))